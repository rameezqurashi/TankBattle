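; Player-controllable tank Blueprint that binds input for camera aiming, firing and driving.
; On BeginPlay it passes the barrel and turret to TankAiming and both tracks to TankMovement.
; Aim axes rotate the azimuth gimbal and spring arm separately for yaw and pitch, and the Fire action calls Fire.
; Throttle axes send forward and right intents to TankMovement instead of driving the tracks directly.
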(event `self.ReceiveBeginPlay`
  ;[1 1 1] Set barrel/turret references
  (`TankAimingComponent.Initialize` (`self.TankAiming`) (`self.TankBarrel`) (`self.TankTurret`))
  (`TankMovementComponent.Initialize` (`self.TankMovement`) (`self.LeftTankTrack`) (`self.RightTankTrack`)))

(event `InputAxis|AimAzimuth`
  (params (AxisValue :type "Float (single-precision)"))
  ;[1 1 1] Aiming/Firing Control
  (`SceneComponent.K2_AddLocalRotation` (`self.AzimuthGimbal`) (`KismetMathLibrary.MakeRotator` 0.0 0.0 AxisValue) false false))

(event `InputAxis|AimElevation`
  (params (AxisValue :type "Float (single-precision)"))
  ;[1 1 1] Aiming/Firing Control
  (`SceneComponent.K2_AddLocalRotation` (`self.SpringArm`) (`KismetMathLibrary.MakeRotator` 0.0 AxisValue) false false))

(event `InputAction|Fire`
  (params (Key :type "Key Structure" :default "AnyKey"))
  ;[1 1 1] Aiming/Firing Control
  (:`Pressed`
    (`self.Fire`)))

(event `InputAxis|RightTrackThrottle`
  (params (AxisValue :type "Float (single-precision)"))
  ;[1 1 1] Movement Input Bindings
  (`TankMovementComponent.IntendMoveRight` (`self.TankMovement`) AxisValue))

(event `InputAxis|ForwardThrottle`
  (params (AxisValue :type "Float (single-precision)"))
  ;[1 1 1] Movement Input Bindings
  (`TankMovementComponent.IntendMoveForward` (`self.TankMovement`) AxisValue))

(fn `UserConstructionScript`)